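; Actor component that records per-frame locations of named bones on a skeletal mesh, taken from the owning Character or supplied through Init.
; BeginPlay preallocates one location array per bone name, sized to a frame limit.
; Start and Stop toggle recording; while active, Tick writes each GetBoneLocation result at the frame counter's index until it passes the limit.
; GetBoneLocation contains an actor-space socket lookup that is left unconnected.
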(event EventTick
  (params (DeltaSeconds :type Float%20%28single-precision%29))
  (bind _sum (Variables|Default|Getsum))
  (if (and (Variables|Default|GetisRecording?) (<= (Variables|Default|Getsum) (Variables|Default|Getlimit)))
    (for (_array_element _array_index) (Variables|Default|GetBoneNames)
      (Utilities|Array|SetArrayElem (.locations (Utilities|Array|Get(acopy) (Variables|Default|GetRecordData) _array_index)) _sum (Utilities|GetBoneLocation _array_element)))
    (Math|Integer|IncrementInt _sum)))

(event EventBeginPlay
  (bind _recorddata (Variables|Default|GetRecordData))
  (Utilities|FlowControl|Sequence
    (:then_0
      (bind _ascharacter (Utilities|Casting|CastToCharacter (Components|GetOwner)))
      (Variables|Default|SetMeshRef (Variables|/Script/Engine.Character|GetMesh _ascharacter)))
    (:then_1
      (for _array_element (Variables|Default|GetBoneNames)
        (bind _returnvalue (Utilities|Array|Add _recorddata (Utilities|Struct|MakeSocketLocationPerFrame)))
        (Utilities|Array|Resize (.locations (Utilities|Array|Get(acopy) _recorddata _returnvalue)) (Variables|Default|Getlimit))))))

(fn Start
  (Variables|Default|Setsum 0)
  (Variables|Default|SetisRecording? true))

(fn Stop
  (Variables|Default|SetisRecording? false))

(fn Init
  (params (skeletal%20mesh%20component :type Skeletal%20Mesh%20Component%20Object%20Reference))
  (Variables|Default|SetMeshRef skeletal%20mesh%20component))
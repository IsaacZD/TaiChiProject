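; Student character for a Tai Chi game that grades how closely its body follows the teacher demo.
; Per-bone overlaps with matching teacher colliders set match flags and hide teacher lights, while Tick accumulates unmatched time during playback.
; When playback stops, DoOnce latches trigger per-bone percentage grades, passed to UserCharacter and TaiChiGameMode, plus a text file of wrong times.
; Touching its own neck with the right hand triggers the user's Interact.
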(event OnComponentBeginOverlap(Stu_Neck)
  (params (OverlappedComponent :type Primitive%20Component%20Object%20Reference) (OtherActor :type Actor%20Object%20Reference) (OtherComp :type Primitive%20Component%20Object%20Reference) (OtherBodyIndex :type Integer) (bFromSweep :type Boolean) (SweepResult :type Hit%20Result%20Structure%20%28by%20ref%29))
  ;[1 1 1] EachBoneCollision
  ;;[1 1 1] Neck
  (CallFunction|BoneCollision OtherComp "Tea_Neck" 13 true))

(event OnComponentBeginOverlap(Stu_LFA)
  (params (OverlappedComponent :type Primitive%20Component%20Object%20Reference) (OtherActor :type Actor%20Object%20Reference) (OtherComp :type Primitive%20Component%20Object%20Reference) (OtherBodyIndex :type Integer) (bFromSweep :type Boolean) (SweepResult :type Hit%20Result%20Structure%20%28by%20ref%29))
  ;[1 1 1] EachBoneCollision
  ;;[1 1 1] LeftForeArm
  (CallFunction|BoneCollision OtherComp "Tea_LFA" 0 true))

(event OnComponentEndOverlap(Stu_RA)
  (params (OverlappedComponent :type Primitive%20Component%20Object%20Reference) (OtherActor :type Actor%20Object%20Reference) (OtherComp :type Primitive%20Component%20Object%20Reference) (OtherBodyIndex :type Integer))
  ;[1 1 1] EachBoneCollision
  ;;[1 1 1] RightArm
  (CallFunction|BoneCollision OtherComp "Tea_RA" 4 false))

(event OnComponentBeginOverlap(Stu_RH)
  (params (OverlappedComponent :type Primitive%20Component%20Object%20Reference) (OtherActor :type Actor%20Object%20Reference) (OtherComp :type Primitive%20Component%20Object%20Reference) (OtherBodyIndex :type Integer) (bFromSweep :type Boolean) (SweepResult :type Hit%20Result%20Structure%20%28by%20ref%29))
  ;[1 1 1] EachBoneCollision
  ;;[1 1 1] RightHand
  (Utilities|Casting|CastToTaiChiGameMode (Game|GetGameMode))
  (if (Utilities|Enum|Equal(Enum) (Utilities|GetObjectName OtherComp) "Stu_Neck")
    (bind _asuser_character (Utilities|Casting|CastToUserCharacter (Game|Player|GetPlayerPawn 0)))
    (Default|Interact _asuser_character)
    (else
      (CallFunction|BoneCollision OtherComp "Tea_RH" 5 true))))

(event OnComponentEndOverlap(Stu_RH)
  (params (OverlappedComponent :type Primitive%20Component%20Object%20Reference) (OtherActor :type Actor%20Object%20Reference) (OtherComp :type Primitive%20Component%20Object%20Reference) (OtherBodyIndex :type Integer))
  ;[1 1 1] EachBoneCollision
  ;;[1 1 1] RightHand
  (CallFunction|BoneCollision OtherComp "Tea_RH" 5 false))

(event OnComponentBeginOverlap(Stu_Head)
  (params (OverlappedComponent :type Primitive%20Component%20Object%20Reference) (OtherActor :type Actor%20Object%20Reference) (OtherComp :type Primitive%20Component%20Object%20Reference) (OtherBodyIndex :type Integer) (bFromSweep :type Boolean) (SweepResult :type Hit%20Result%20Structure%20%28by%20ref%29))
  ;[1 1 1] EachBoneCollision
  ;;[1 1 1] Head
  (CallFunction|BoneCollision OtherComp "Tea_Head" 12 true))

(event OnComponentEndOverlap(Stu_Head)
  (params (OverlappedComponent :type Primitive%20Component%20Object%20Reference) (OtherActor :type Actor%20Object%20Reference) (OtherComp :type Primitive%20Component%20Object%20Reference) (OtherBodyIndex :type Integer))
  ;[1 1 1] EachBoneCollision
  ;;[1 1 1] Head
  (CallFunction|BoneCollision OtherComp "Tea_Head" 12 false))

(event OnComponentBeginOverlap(Stu_LUL)
  (params (OverlappedComponent :type Primitive%20Component%20Object%20Reference) (OtherActor :type Actor%20Object%20Reference) (OtherComp :type Primitive%20Component%20Object%20Reference) (OtherBodyIndex :type Integer) (bFromSweep :type Boolean) (SweepResult :type Hit%20Result%20Structure%20%28by%20ref%29))
  ;[1 1 1] EachBoneCollision
  ;;[1 1 1] LeftUpLeg
  (CallFunction|BoneCollision OtherComp "Tea_LUL" 6 true))

(event OnComponentEndOverlap(Stu_LUL)
  (params (OverlappedComponent :type Primitive%20Component%20Object%20Reference) (OtherActor :type Actor%20Object%20Reference) (OtherComp :type Primitive%20Component%20Object%20Reference) (OtherBodyIndex :type Integer))
  ;[1 1 1] EachBoneCollision
  ;;[1 1 1] LeftUpLeg
  (CallFunction|BoneCollision OtherComp "Tea_LUL" 6 false))

(event OnComponentBeginOverlap(Stu_LL)
  (params (OverlappedComponent :type Primitive%20Component%20Object%20Reference) (OtherActor :type Actor%20Object%20Reference) (OtherComp :type Primitive%20Component%20Object%20Reference) (OtherBodyIndex :type Integer) (bFromSweep :type Boolean) (SweepResult :type Hit%20Result%20Structure%20%28by%20ref%29))
  ;[1 1 1] EachBoneCollision
  ;;[1 1 1] LeftLeg
  (CallFunction|BoneCollision OtherComp "Tea_LL" 7 true))

(event OnComponentEndOverlap(Stu_LL)
  (params (OverlappedComponent :type Primitive%20Component%20Object%20Reference) (OtherActor :type Actor%20Object%20Reference) (OtherComp :type Primitive%20Component%20Object%20Reference) (OtherBodyIndex :type Integer))
  ;[1 1 1] EachBoneCollision
  ;;[1 1 1] LeftLeg
  (CallFunction|BoneCollision OtherComp "Tea_LL" 7 false))

(event OnComponentBeginOverlap(Stu_LF)
  (params (OverlappedComponent :type Primitive%20Component%20Object%20Reference) (OtherActor :type Actor%20Object%20Reference) (OtherComp :type Primitive%20Component%20Object%20Reference) (OtherBodyIndex :type Integer) (bFromSweep :type Boolean) (SweepResult :type Hit%20Result%20Structure%20%28by%20ref%29))
  ;[1 1 1] EachBoneCollision
  ;;[1 1 1] LeftFoot
  (CallFunction|BoneCollision OtherComp "Tea_LF" 8 true))

(event OnComponentEndOverlap(Stu_LFA)
  (params (OverlappedComponent :type Primitive%20Component%20Object%20Reference) (OtherActor :type Actor%20Object%20Reference) (OtherComp :type Primitive%20Component%20Object%20Reference) (OtherBodyIndex :type Integer))
  ;[1 1 1] EachBoneCollision
  ;;[1 1 1] LeftForeArm
  (CallFunction|BoneCollision OtherComp "Tea_LFA" 0 false))

(event OnComponentEndOverlap(Stu_LF)
  (params (OverlappedComponent :type Primitive%20Component%20Object%20Reference) (OtherActor :type Actor%20Object%20Reference) (OtherComp :type Primitive%20Component%20Object%20Reference) (OtherBodyIndex :type Integer))
  ;[1 1 1] EachBoneCollision
  ;;[1 1 1] LeftFoot
  (CallFunction|BoneCollision OtherComp "Tea_LF" 8 false))

(event OnComponentBeginOverlap(Stu_RUL)
  (params (OverlappedComponent :type Primitive%20Component%20Object%20Reference) (OtherActor :type Actor%20Object%20Reference) (OtherComp :type Primitive%20Component%20Object%20Reference) (OtherBodyIndex :type Integer) (bFromSweep :type Boolean) (SweepResult :type Hit%20Result%20Structure%20%28by%20ref%29))
  ;[1 1 1] EachBoneCollision
  ;;[1 1 1] RightUpLeg
  (CallFunction|BoneCollision OtherComp "Tea_RUL" 9 true))

(event OnComponentEndOverlap(Stu_RUL)
  (params (OverlappedComponent :type Primitive%20Component%20Object%20Reference) (OtherActor :type Actor%20Object%20Reference) (OtherComp :type Primitive%20Component%20Object%20Reference) (OtherBodyIndex :type Integer))
  ;[1 1 1] EachBoneCollision
  ;;[1 1 1] RightUpLeg
  (CallFunction|BoneCollision OtherComp "Tea_RUL" 9 false))

(event OnComponentBeginOverlap(Stu_RL)
  (params (OverlappedComponent :type Primitive%20Component%20Object%20Reference) (OtherActor :type Actor%20Object%20Reference) (OtherComp :type Primitive%20Component%20Object%20Reference) (OtherBodyIndex :type Integer) (bFromSweep :type Boolean) (SweepResult :type Hit%20Result%20Structure%20%28by%20ref%29))
  ;[1 1 1] EachBoneCollision
  ;;[1 1 1] RightLeg
  (CallFunction|BoneCollision OtherComp "Tea_RL" 10 true))

(event OnComponentEndOverlap(Stu_RL)
  (params (OverlappedComponent :type Primitive%20Component%20Object%20Reference) (OtherActor :type Actor%20Object%20Reference) (OtherComp :type Primitive%20Component%20Object%20Reference) (OtherBodyIndex :type Integer))
  ;[1 1 1] EachBoneCollision
  ;;[1 1 1] RightLeg
  (CallFunction|BoneCollision OtherComp "Tea_RL" 10 false))

(event OnComponentBeginOverlap(Stu_RF)
  (params (OverlappedComponent :type Primitive%20Component%20Object%20Reference) (OtherActor :type Actor%20Object%20Reference) (OtherComp :type Primitive%20Component%20Object%20Reference) (OtherBodyIndex :type Integer) (bFromSweep :type Boolean) (SweepResult :type Hit%20Result%20Structure%20%28by%20ref%29))
  ;[1 1 1] EachBoneCollision
  ;;[1 1 1] RightFoot
  (CallFunction|BoneCollision OtherComp "Tea_RF" 11 true))

(event OnComponentEndOverlap(Stu_RF)
  (params (OverlappedComponent :type Primitive%20Component%20Object%20Reference) (OtherActor :type Actor%20Object%20Reference) (OtherComp :type Primitive%20Component%20Object%20Reference) (OtherBodyIndex :type Integer))
  ;[1 1 1] EachBoneCollision
  ;;[1 1 1] RightFoot
  (CallFunction|BoneCollision OtherComp "Tea_RF" 11 false))

(event OnComponentBeginOverlap(Stu_LA)
  (params (OverlappedComponent :type Primitive%20Component%20Object%20Reference) (OtherActor :type Actor%20Object%20Reference) (OtherComp :type Primitive%20Component%20Object%20Reference) (OtherBodyIndex :type Integer) (bFromSweep :type Boolean) (SweepResult :type Hit%20Result%20Structure%20%28by%20ref%29))
  ;[1 1 1] EachBoneCollision
  ;;[1 1 1] LeftArm
  (CallFunction|BoneCollision OtherComp "Tea_LA" 1 true))

(event OnComponentEndOverlap(Stu_LA)
  (params (OverlappedComponent :type Primitive%20Component%20Object%20Reference) (OtherActor :type Actor%20Object%20Reference) (OtherComp :type Primitive%20Component%20Object%20Reference) (OtherBodyIndex :type Integer))
  ;[1 1 1] EachBoneCollision
  ;;[1 1 1] LeftArm
  (CallFunction|BoneCollision OtherComp "Tea_LA" 1 false))

(event OnComponentBeginOverlap(Stu_LH)
  (params (OverlappedComponent :type Primitive%20Component%20Object%20Reference) (OtherActor :type Actor%20Object%20Reference) (OtherComp :type Primitive%20Component%20Object%20Reference) (OtherBodyIndex :type Integer) (bFromSweep :type Boolean) (SweepResult :type Hit%20Result%20Structure%20%28by%20ref%29))
  ;[1 1 1] EachBoneCollision
  ;;[1 1 1] LeftHand
  (CallFunction|BoneCollision OtherComp "Tea_LH" 2 true))

(event OnComponentEndOverlap(Stu_LH)
  (params (OverlappedComponent :type Primitive%20Component%20Object%20Reference) (OtherActor :type Actor%20Object%20Reference) (OtherComp :type Primitive%20Component%20Object%20Reference) (OtherBodyIndex :type Integer))
  ;[1 1 1] EachBoneCollision
  ;;[1 1 1] LeftHand
  (CallFunction|BoneCollision OtherComp "Tea_LH" 2 false))

(event OnComponentBeginOverlap(Stu_RFA)
  (params (OverlappedComponent :type Primitive%20Component%20Object%20Reference) (OtherActor :type Actor%20Object%20Reference) (OtherComp :type Primitive%20Component%20Object%20Reference) (OtherBodyIndex :type Integer) (bFromSweep :type Boolean) (SweepResult :type Hit%20Result%20Structure%20%28by%20ref%29))
  ;[1 1 1] EachBoneCollision
  ;;[1 1 1] RightForeArm
  (CallFunction|BoneCollision OtherComp "Tea_RFA" 3 true))

(event OnComponentEndOverlap(Stu_Neck)
  (params (OverlappedComponent :type Primitive%20Component%20Object%20Reference) (OtherActor :type Actor%20Object%20Reference) (OtherComp :type Primitive%20Component%20Object%20Reference) (OtherBodyIndex :type Integer))
  ;[1 1 1] EachBoneCollision
  ;;[1 1 1] Neck
  (CallFunction|BoneCollision OtherComp "Tea_Neck" 13 false))

(event OnComponentBeginOverlap(Stu_LS)
  (params (OverlappedComponent :type Primitive%20Component%20Object%20Reference) (OtherActor :type Actor%20Object%20Reference) (OtherComp :type Primitive%20Component%20Object%20Reference) (OtherBodyIndex :type Integer) (bFromSweep :type Boolean) (SweepResult :type Hit%20Result%20Structure%20%28by%20ref%29))
  ;[1 1 1] EachBoneCollision
  ;;[1 1 1] LeftShoulder
  (CallFunction|BoneCollision OtherComp "Tea_LS" 14 true))

(event OnComponentEndOverlap(Stu_RFA)
  (params (OverlappedComponent :type Primitive%20Component%20Object%20Reference) (OtherActor :type Actor%20Object%20Reference) (OtherComp :type Primitive%20Component%20Object%20Reference) (OtherBodyIndex :type Integer))
  ;[1 1 1] EachBoneCollision
  ;;[1 1 1] RightForeArm
  (CallFunction|BoneCollision OtherComp "Tea_RFA" 3 false))

(event OnComponentEndOverlap(Stu_LS)
  (params (OverlappedComponent :type Primitive%20Component%20Object%20Reference) (OtherActor :type Actor%20Object%20Reference) (OtherComp :type Primitive%20Component%20Object%20Reference) (OtherBodyIndex :type Integer))
  ;[1 1 1] EachBoneCollision
  ;;[1 1 1] LeftShoulder
  (CallFunction|BoneCollision OtherComp "Tea_LS" 14 false))

(event OnComponentBeginOverlap(Stu_RS)
  (params (OverlappedComponent :type Primitive%20Component%20Object%20Reference) (OtherActor :type Actor%20Object%20Reference) (OtherComp :type Primitive%20Component%20Object%20Reference) (OtherBodyIndex :type Integer) (bFromSweep :type Boolean) (SweepResult :type Hit%20Result%20Structure%20%28by%20ref%29))
  ;[1 1 1] EachBoneCollision
  ;;[1 1 1] RightShoulder
  (CallFunction|BoneCollision OtherComp "Tea_RS" 15 true))

(event OnComponentEndOverlap(Stu_RS)
  (params (OverlappedComponent :type Primitive%20Component%20Object%20Reference) (OtherActor :type Actor%20Object%20Reference) (OtherComp :type Primitive%20Component%20Object%20Reference) (OtherBodyIndex :type Integer))
  ;[1 1 1] EachBoneCollision
  ;;[1 1 1] RightShoulder
  (CallFunction|BoneCollision OtherComp "Tea_RS" 15 false))

(event OnComponentBeginOverlap(Stu_RA)
  (params (OverlappedComponent :type Primitive%20Component%20Object%20Reference) (OtherActor :type Actor%20Object%20Reference) (OtherComp :type Primitive%20Component%20Object%20Reference) (OtherBodyIndex :type Integer) (bFromSweep :type Boolean) (SweepResult :type Hit%20Result%20Structure%20%28by%20ref%29))
  ;[1 1 1] EachBoneCollision
  ;;[1 1 1] RightArm
  (CallFunction|BoneCollision OtherComp "Tea_RA" 4 true))

(event Custom|LocationTest
  ;[1 1 1] LocationTest
  (Variables|Default|Setlocation1 (Class|SavetoTxt|StringAdd (Class|SavetoTxt|StringAdd (Class|SavetoTxt|StringAdd (Class|SavetoTxt|StringAdd (Variables|Default|Getlocation1) (Utilities|String|ToString(Vector) (.Location (Math|Transform|BreakTransform (Transformation|GetSocketTransform (Variables|Character|GetMesh) "LeftForeArm" "RTS_Component"))))) "             ") (Utilities|String|ToString(Integer) (Variables|Default|GetFrameNumber))) " 
"))
  (Variables|Default|Setlocation2 (Class|SavetoTxt|StringAdd (Class|SavetoTxt|StringAdd (Class|SavetoTxt|StringAdd (Class|SavetoTxt|StringAdd (Variables|Default|Getlocation1) (Utilities|String|ToString(Vector) (.Location (Math|Transform|BreakTransform (Transformation|GetSocketTransform (Variables|/Script/Engine.Character|GetMesh (Variables|Default|GetTeacherDemoRef)) "LeftForeArm" "RTS_Actor"))))) "             ") (Utilities|String|ToString(Integer) (Variables|Default|GetFrameNumber))) " 
")))

(event Custom|SumWrongTime
  (bind _wrongtime (Variables|Default|GetWrongTime))
  ;[1 1 1] SumWrongTime
  (for (_array_element _array_index) (Variables|Default|GetBoneBools)
    (if (not _array_element)
      (Utilities|Array|SetArrayElem _wrongtime _array_index (+ (Utilities|Array|Get(acopy) _wrongtime _array_index) (Variables|Default|GetDeltaSeconds))))))

(event Custom|OutputTxt
  ;[1 1 1] OutputTxt
  (for _array_element (Variables|Default|GetWrongTime)
    (Variables|Default|SetOutput (Utilities|String|Append (Variables|Default|GetOutput) (Utilities|String|ToString(Float) _array_element) " 
")))
  (for (_array_element_2 _array_index) (Variables|Default|GetBoneNames)
    (Variables|Default|SetOutput (Utilities|String|Append (Variables|Default|GetOutput) _array_element_2 ":" (Utilities|String|ToString(Float) (Utilities|Array|Get(acopy) (Variables|Default|GetWrongTime) _array_index)) " 
")))
  ;[1 1 1] ComputeGrades
  (Class|SavetoTxt|FileSaveString (Variables|Default|GetOutput) "Temp\\output.txt")
  (Variables|Default|SetHaveFinished true))

(event Custom|ComputeGrades
  (bind _teacherdemoref (Variables|Default|GetTeacherDemoRef))
  (bind _teamtg (Variables|/Game/Blueprints/Pawns/TeacherDemoCharacter.TeacherDemoCharacter_C|GetTeaMtg _teacherdemoref))
  (bind _sequencelength (Variables|/Script/Engine.AnimSequenceBase|GetSequenceLength _teamtg))
  ;[1 1 1] ComputeGrades
  ;;[1 1 1] OutputTxt
  (for (_ _array_index) (Variables|Default|GetGrades)
    (Utilities|Array|SetArrayElem (Variables|Default|GetGrades) _array_index 0 true))
  (for (_array_element _array_index_2) (Variables|Default|GetWrongTime)
    (Utilities|Array|SetArrayElem (Variables|Default|GetGrades) _array_index_2 (Math|Float|Round (* (/ (- _sequencelength _array_element) _sequencelength) 1e+02)) true))
  (Variables|Default|SetHaveFinished true)
  (bind _asuser_character (Utilities|Casting|CastToUserCharacter (Game|Player|GetPlayerPawn 0)))
  (Variables|/Game/Blueprints/Pawns/UserCharacter.UserCharacter_C|SetGrades _asuser_character (Variables|Default|GetGrades)))

(event EventBeginPlay
  (bind _self self)
  (bind _mesh (Variables|Character|GetMesh))
  (Transformation|SetActorLocation _self (- (Transformation|GetActorLocation _self) "0, 0,200.000000") false false)
  (bind _astai_chi_game_mode (Utilities|Casting|CastToTaiChiGameMode (Game|GetGameMode)))
  (Variables|/Game/FirstPersonBP/Blueprints/TaiChiGameMode.TaiChiGameMode_C|SetStudentRef _astai_chi_game_mode self)
  (Rendering|SetRenderCustomDepth _mesh (not (Variables|/Script/Engine.PrimitiveComponent|GetbRenderCustomDepth _mesh))))

(event EventTick
  (params (DeltaSeconds :type Float%20%28single-precision%29))
  (bind _teacherdemoref (Variables|Default|GetTeacherDemoRef))
  (if (Utilities|IsValid _teacherdemoref)
    (if (Variables|/Game/Blueprints/Pawns/TeacherDemoCharacter.TeacherDemoCharacter_C|GetisPlaying _teacherdemoref)
      (Variables|Default|SetDeltaSeconds DeltaSeconds)
      (CallFunction|SumWrongTime)
      (Utilities|FlowControl|DoOnce false :!label _label
        (:Completed
          (goto _label_2 Reset)))
      (else
        (Utilities|FlowControl|Sequence
          (:then_0
            (Utilities|FlowControl|DoOnce true :!label _label_2
              (:Completed
                (CallFunction|ComputeGrades)
                (CallFunction|OutputTxt)
                (bind _astai_chi_game_mode (Utilities|Casting|CastToTaiChiGameMode (Game|GetGameMode)))
                (Default|UpdateEndRetime _astai_chi_game_mode (Variables|Default|GetGrades)))))
          (:then_1
            (goto _label Reset)))))))

(fn ConstructionScript
  (bind _mesh (Variables|Character|GetMesh))
  ;[1 1 1] Real Time
  (Class|SkinnedMeshComponent|SetSkeletalMesh _mesh "/Game/Characters/FormalStudent/FormalStudent.FormalStudent" true)
  (Components|Animation|SetAnimationMode _mesh "AnimationBlueprint")
  (Components|SkeletalMesh|SetAnimInstanceClass _mesh "/Game/Characters/FormalStudent/FormalStudent_Skeleton_AnimBlueprint.FormalStudent_Skeleton_AnimBlueprint_C"))

(fn GetBoneLocation
  (params (boneName :type String))
  (return (.Location (Math|Transform|BreakTransform (Transformation|GetSocketTransform (Variables|Character|GetMesh) (Utilities|String|StringToName boneName) "RTS_Actor")))))

(fn ComputeDistancebyName
  (params (BoneName :type String))
  (bind _location (Default|GetBoneLocation (Variables|Default|GetTeacherDemoRef) BoneName))
  (bind _location_2 (CallFunction|GetBoneLocation BoneName))
  (return (Math|Vector|VectorLength (- _location_2 _location))))

(fn BoneCollision
  (params (OtherComp :type Primitive%20Component%20Object%20Reference) (BoneName :type String) (Index :type Integer) (IsBegin :type Boolean))
  (bind _bonebools (Variables|Default|GetBoneBools))
  (bind _teacherdemoref (Variables|Default|GetTeacherDemoRef))
  (bind _invesibleteacher (Variables|Default|GetInvesibleTeacher))
  (if (Utilities|Enum|Equal(Enum) (Utilities|GetObjectName OtherComp) BoneName)
    (if IsBegin
      (Utilities|Array|SetArrayElem _bonebools Index true)
      (Default|HideLight _teacherdemoref true Index)
      (Default|HideLight _invesibleteacher true Index)
      (else
        (Utilities|Array|SetArrayElem _bonebools Index false)
        (Default|HideLight _teacherdemoref false Index)
        (Default|HideLight _invesibleteacher false Index)))))

(fn GetGrades
  (return (Variables|Default|GetGrades)))
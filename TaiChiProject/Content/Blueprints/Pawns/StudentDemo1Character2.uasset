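; Student demo character that plays a montage and provides tools for scoring its pose against a teacher demo character.
; Construction applies the Avatar mesh and animation Blueprint, and helpers measure per-bone distance to the teacher.
; Events accumulate wrong time for bones flagged false and save totals to a text file, though Tick is empty here.
; Right-hand overlap with the student's head fires Interact then UnInteract on the player's UserCharacter.
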(event OnComponentBeginOverlap(Stu_RH)
  (params (OverlappedComponent :type Primitive%20Component%20Object%20Reference) (OtherActor :type Actor%20Object%20Reference) (OtherComp :type Primitive%20Component%20Object%20Reference) (OtherBodyIndex :type Integer) (bFromSweep :type Boolean) (SweepResult :type Hit%20Result%20Structure%20%28by%20ref%29))
  ;[1 1 1] LeftMouse
  (if (Utilities|Enum|Equal(Enum) (Utilities|GetObjectName OtherComp) "Stu_Head")
    (bind _asuser_character (Utilities|Casting|CastToUserCharacter (Game|Player|GetPlayerPawn 0)))
    (Default|Interact _asuser_character)
    (Default|UnInteract _asuser_character)))

(event OnComponentEndOverlap(Stu_RH)
  (params (OverlappedComponent :type Primitive%20Component%20Object%20Reference) (OtherActor :type Actor%20Object%20Reference) (OtherComp :type Primitive%20Component%20Object%20Reference) (OtherBodyIndex :type Integer))
  ;[1 1 1] LeftMouse
  (if (Utilities|Enum|Equal(Enum) (Utilities|GetObjectName OtherComp) "Stu_Head")
    _))

(event Custom|LocationTest
  ;[1 1 1] LocationTest
  (Variables|Default|Setlocation1 (Class|SavetoTxt|StringAdd (Class|SavetoTxt|StringAdd (Class|SavetoTxt|StringAdd (Class|SavetoTxt|StringAdd (Variables|Default|Getlocation1) (Utilities|String|ToString(Vector) (.Location (Math|Transform|BreakTransform (Transformation|GetSocketTransform (Variables|Character|GetMesh) "LeftForeArm" "RTS_Component"))))) "             ") (Utilities|String|ToString(Integer) (Variables|Default|GetFrameNumber))) " 
"))
  (Variables|Default|Setlocation2 (Class|SavetoTxt|StringAdd (Class|SavetoTxt|StringAdd (Class|SavetoTxt|StringAdd (Class|SavetoTxt|StringAdd (Variables|Default|Getlocation1) (Utilities|String|ToString(Vector) (.Location (Math|Transform|BreakTransform (Transformation|GetSocketTransform (Variables|/Script/Engine.Character|GetMesh (Variables|Default|GetTeacherDemoRef)) "LeftForeArm" "RTS_Actor"))))) "             ") (Utilities|String|ToString(Integer) (Variables|Default|GetFrameNumber))) " 
")))

(event Custom|SumWrongTime
  (bind _wrongtime (Variables|Default|GetWrongTime))
  ;[1 1 1] SumWrongTime
  (for (_array_element _array_index) (Variables|Default|GetBoneBools)
    (if (not _array_element)
      (Utilities|Array|SetArrayElem _wrongtime _array_index (+ (Utilities|Array|Get(acopy) _wrongtime _array_index) (Variables|Default|GetDeltaSeconds))))))

(event Custom|OutputTxt
  ;[1 1 1] OutputTxt
  (for (_array_element _array_index) (Variables|Default|GetBoneNames)
    (Variables|Default|SetOutput (Utilities|String|Append (Variables|Default|GetOutput) _array_element ":" (Utilities|String|ToString(Float) (Utilities|Array|Get(acopy) (Variables|Default|GetWrongTime) _array_index)) " 
")))
  (Class|SavetoTxt|FileSaveString (Variables|Default|GetOutput) "Temp\\output.txt")
  (Variables|Default|SetHaveFinished true))

(event EventBeginPlay
  (Animation|PlayAnimMontage (Variables|Default|GetAnimMontage) 1.0 "None"))

(event Collision|EventActorBeginOverlap
  (params (OtherActor :type Actor%20Object%20Reference)))

(event EventTick
  (params (DeltaSeconds :type Float%20%28single-precision%29)))

(fn ConstructionScript
  (bind _mesh (Variables|Character|GetMesh))
  ;[1 1 1] Real Time
  (Class|SkinnedMeshComponent|SetSkeletalMesh _mesh "/Game/Avatar/Avatar.Avatar" true)
  (Components|Animation|SetAnimationMode _mesh "AnimationBlueprint")
  (Components|SkeletalMesh|SetAnimInstanceClass _mesh "/Game/Avatar/Avatar_Skeleton_AnimBlueprint.Avatar_Skeleton_AnimBlueprint_C"))

(fn GetBoneLocation
  (params (boneName :type String))
  (return (.Location (Math|Transform|BreakTransform (Transformation|GetSocketTransform (Variables|Character|GetMesh) (Utilities|String|StringToName boneName) "RTS_Actor")))))

(fn ComputeDistancebyName
  (params (BoneName :type String))
  (bind _location (Default|GetBoneLocation (Variables|Default|GetTeacherDemoRef) BoneName))
  (bind _location_2 (CallFunction|GetBoneLocation BoneName))
  (return (Math|Vector|VectorLength (- _location_2 _location))))
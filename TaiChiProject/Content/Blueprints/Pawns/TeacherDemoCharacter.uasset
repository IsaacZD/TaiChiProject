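; Teacher demo character that plays montages of eight individual moves or a combined whole sequence.
; UpdateMtg selects the montage by index, and two play events start it on the mesh, guarded by an IsPlaying flag or a DoOnce in the watch variant.
; The construction script collects per-body-part visual components into a Bones array, which HideLight shows or hides by index.
; GetBoneLocation returns a named bone's location in actor space.
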(event Custom|TeaMtgPlay
  (if (not (Variables|Default|GetisPlaying))
    (Variables|Default|SetisPlaying true)
    (Animation|Montage|MontagePlay (Components|SkeletalMesh|GetAnimInstance (Variables|Character|GetMesh)) (Variables|Default|GetTeaMtg) 1.0 "MontageLength" 0.0)))

(event Custom|TeaMtgPlayInWatch
  (Variables|Default|SetisPlaying true)
  (Utilities|FlowControl|DoOnce false
    (:Completed
      (Animation|Montage|MontagePlay (Components|SkeletalMesh|GetAnimInstance (Variables|Character|GetMesh)) (Variables|Default|GetTeaMtg) 1.0 "MontageLength" 0.0))))

(event Custom|UpdateMtg
  (params (WhichMove :type Integer))
  (bind _output_get (Variables|Default|SetWhichMove WhichMove))
  (switch int _output_get
    (:0
      (Variables|Default|SetTeaMtg "/Game/Animations/FormalAnim/move_1_Anim_Montage.move_1_Anim_Montage"))
    (:1
      (Variables|Default|SetTeaMtg "/Game/Animations/FormalAnim/move_2_Anim_Montage.move_2_Anim_Montage"))
    (:2
      (Variables|Default|SetTeaMtg "/Game/Animations/FormalAnim/move_3_Anim_Montage.move_3_Anim_Montage"))
    (:3
      (Variables|Default|SetTeaMtg "/Game/Animations/FormalAnim/move_4_Anim_Montage.move_4_Anim_Montage"))
    (:4
      (Variables|Default|SetTeaMtg "/Game/Animations/FormalAnim/move_5_Anim_Montage.move_5_Anim_Montage"))
    (:5
      (Variables|Default|SetTeaMtg "/Game/Animations/FormalAnim/move_6_Anim_Montage.move_6_Anim_Montage"))
    (:6
      (Variables|Default|SetTeaMtg "/Game/Animations/FormalAnim/move_7_Anim_Montage.move_7_Anim_Montage"))
    (:7
      (Variables|Default|SetTeaMtg "/Game/Animations/FormalAnim/move_8_Anim_Montage.move_8_Anim_Montage"))
    (:8
      (Variables|Default|SetTeaMtg "/Game/Animations/FormalAnim/move_whole8_Anim_Montage.move_whole8_Anim_Montage"))))

(event EventBeginPlay)

(fn ConstructionScript
  (Utilities|Array|Add (Variables|Default|GetBones) (Variables|Default|GetVisibleTea_LFA))
  (Utilities|Array|Add (Variables|Default|GetBones) (Variables|Default|GetVisibleTea_LA))
  (Utilities|Array|Add (Variables|Default|GetBones) (Variables|Default|GetVisibleTea_LH))
  (Utilities|Array|Add (Variables|Default|GetBones) (Variables|Default|GetVisibleTea_RFA))
  (Utilities|Array|Add (Variables|Default|GetBones) (Variables|Default|GetVisibleTea_RA))
  (Utilities|Array|Add (Variables|Default|GetBones) (Variables|Default|GetVisibleTea_RH))
  (Utilities|Array|Add (Variables|Default|GetBones) (Variables|Default|GetVisibleTea_Head))
  (Utilities|Array|Add (Variables|Default|GetBones) (Variables|Default|GetVisibleTea_LUL))
  (Utilities|Array|Add (Variables|Default|GetBones) (Variables|Default|GetVisibleTea_LL))
  (Utilities|Array|Add (Variables|Default|GetBones) (Variables|Default|GetVisibleTea_LF))
  (Utilities|Array|Add (Variables|Default|GetBones) (Variables|Default|GetVisibleTea_RUL))
  (Utilities|Array|Add (Variables|Default|GetBones) (Variables|Default|GetVisibleTea_RL))
  (Utilities|Array|Add (Variables|Default|GetBones) (Variables|Default|GetVisibleTea_RF))
  (Utilities|Array|Add (Variables|Default|GetBones) (Variables|Default|GetVisibleTea_Neck))
  (Utilities|Array|Add (Variables|Default|GetBones) (Variables|Default|GetVisibleTea_LS))
  (Utilities|Array|Add (Variables|Default|GetBones) (Variables|Default|GetVisibleTea_RS))
  (Utilities|Array|Add (Variables|Default|GetBones) 0))

(fn GetBoneLocation
  (params (boneName :type String))
  (return (.Location (Math|Transform|BreakTransform (Transformation|GetSocketTransform (Variables|Character|GetMesh) (Utilities|String|StringToName boneName) "RTS_Actor")))))

(fn HideLight
  (params (Hidden :type Boolean) (Index :type Integer))
  (bind _bones (Variables|Default|GetBones))
  (bind _output (Utilities|Array|Get(acopy) _bones Index))
  (if Hidden
    (Development|SetHiddeninGame _output true false)
    (else
      (Development|SetHiddeninGame _output false false))))